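; First-person player Blueprint that carries the weapon inventory, creates the HUD and handles player death.
; Equipped guns attach to GunPosition and are stored by type, with an ordered list for cycling; switching shows only the current gun and updates the HUD.
; Shooting and ammo calls are forwarded to weapons as messages, with a BPI_Gun check before ammo-capacity queries.
; Hit zeroes HP regardless of damage, then shows game over and pauses.
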(event `self.ReceiveBeginPlay`
  (bind _returnvalue (`|CreateWidget` "/Game/UI/Blueprints/WBP_PlayerHUD.WBP_PlayerHUD_C" null self))
  (bind _output_get (set `self.PlayerHUD` _returnvalue))
  (`UserWidget.AddToViewport` _output_get 0))

(event `/Game/Blueprints/Interfaces/BPI_Player.EquipWeapon`
  (params (Type :type "/Game/Blueprints/E_WeaponType Enum" :default "NewEnumerator0") (WeaponActor :type "/Game/Blueprints/Guns/BP_WeaponBase Object Reference"))
  (if (`BlueprintMapLibrary.Map_Contains` (`self.Weapons`) Type)
    (`KismetSystemLibrary.PrintString` "Gun already equipped")
    (else
      (`BlueprintMapLibrary.Map_Add` (`self.Weapons`) Type WeaponActor)
      (`KismetArrayLibrary.Array_Add` (`self.WeaponTypes`) Type)
      (`self.K2_AttachToComponent` WeaponActor (`self.Gun Position`) "None" "SnapToTarget" "SnapToTarget" "KeepRelative" true)
      (`self.SetCurrentWeapon` Type))))

(event `/Game/Blueprints/Interfaces/BPI_Player.CycleWeapon`
  (`self.SetCurrentWeapon` (`|GetArrayItem` (`self.WeaponTypes`) (mod (+ (`self.CurrentWeaponID`) 1) (`KismetArrayLibrary.Array_Length` (`self.WeaponTypes`))))))

(event `/Game/Blueprints/Interfaces/BPI_Player.Shoot`
  (message `/Game/Blueprints/Interfaces/BPI_Gun.Shoot` (`self.CurrentWeapon`)))

(event `/Game/Blueprints/Interfaces/BPI_Player.AddAmmoIntoWeapon`
  (params (WeaponType :type "/Game/Blueprints/E_WeaponType Enum" :default "NewEnumerator0") (NewAmmo :type Integer))
  (message `/Game/Blueprints/Interfaces/BPI_Gun.AddAmmo` (`BlueprintMapLibrary.Map_Find` (`self.Weapons`) WeaponType) NewAmmo))

(event `End Game`
  (bind _returnvalue (`GameplayStatics.GetPlayerController` 0))
  (`KismetSystemLibrary.PrintString` "Player ded" true true (struct :`R` 1.0 :`A` 1.0) 30.0)
  (bind _returnvalue_2 (`|CreateWidget` "/Game/UI/Blueprints/WBP_GameOver.WBP_GameOver_C"))
  (`UserWidget.AddToViewport` _returnvalue_2 0)
  (`WidgetBlueprintLibrary.SetInputMode_UIOnlyEx` _returnvalue null)
  (`GameplayStatics.SetGamePaused` true)
  (set `PlayerController.bShowMouseCursor` true _returnvalue))

(fn `CanAddAmmoIntoWeapon`
  (params (Type :type "/Game/Blueprints/E_WeaponType Enum" :default "NewEnumerator0") (NewAmmo :type Integer))
  (returns (CanAddAmmo :type Boolean))
  (bind _value (`BlueprintMapLibrary.Map_Find` (`self.Weapons`) Type))
  (bind _hasweapon (`/Game/Blueprints/Interfaces/BPI_Player.HasWeaponOfType` Type))
  (if _hasweapon
    (if (`KismetSystemLibrary.DoesImplementInterface` _value "/Game/Blueprints/Interfaces/BPI_Gun.BPI_Gun_C")
      (bind _canaddammo (message `/Game/Blueprints/Interfaces/BPI_Gun.CanAddAmmoIntoWeapon` _value NewAmmo))
      (return _canaddammo)
      (else
        _)))
  (return false))

(fn `HasWeaponOfType`
  (params (Type :type "/Game/Blueprints/E_WeaponType Enum" :default "NewEnumerator0"))
  (returns (HasWeapon :type Boolean))
  (return (`BlueprintMapLibrary.Map_Contains` (`self.Weapons`) Type)))

(fn `HideAllWeapons`
  (bind _keys (`BlueprintMapLibrary.Map_Keys` (`self.Weapons`)))
  (for _array_element _keys
    (bind _value (`BlueprintMapLibrary.Map_Find` (`self.Weapons`) _array_element))
    (`self.SetActorEnableCollision` _value false)
    (`self.SetActorHiddenInGame` _value true)))

(fn `Hit`
  (params (Damage :type Integer))
  (returns (XPReward :type Integer))
  (set `self.HP` 0)
  (`self.End Game`)
  (return 0))

(fn `SetCurrentWeapon`
  (params (Weapon :type "/Game/Blueprints/E_WeaponType Enum" :default "NewEnumerator0"))
  (bind (_value _returnvalue) (`BlueprintMapLibrary.Map_Find` (`self.Weapons`) Weapon))
  (if (not _returnvalue)
    (`KismetSystemLibrary.PrintString` "Cannot switch to selected weapon!")
    (else
      (`|ExecutionSequence`
        (:`then_0`
          (`self.HideAllWeapons`))
        (:`then_1`
          (`self.SetActorEnableCollision` _value true)
          (`self.SetActorHiddenInGame` _value false))
        (:`then_2`
          (set `self.CurrentWeapon` _value))
        (:`then_3`
          (set `self.CurrentWeaponID` (`KismetArrayLibrary.Array_Find` (`self.WeaponTypes`) Weapon)))
        (:`then_4`
          (`/Game/UI/Blueprints/WBP_PlayerHUD.ChangeWeapon` (`self.PlayerHUD`) Weapon))))))

(fn `UserConstructionScript`)
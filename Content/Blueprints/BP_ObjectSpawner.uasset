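; BP_ObjectSpawner populates the level with weapons and crates when play begins.
; It gathers every BP_SpawnPoint actor and shuffles the list to randomize placement.
; Each entry in WeaponTypes spawns once at its own point, then every remaining point receives a random pick from CrateTypes.
; A shared SpawnAt event spawns the chosen class at the indexed point's transform.
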(event `self.ReceiveBeginPlay`
  (bind _outactors (`GameplayStatics.GetAllActorsOfClass` "/Game/Blueprints/BP_SpawnPoint.BP_SpawnPoint_C"))
  (bind _output_get (set `self.Locations` _outactors))
  (`KismetArrayLibrary.Array_Shuffle` _output_get)
  (`|ExecutionSequence`
    (:`then_0`
      (for (_array_element _array_index) (`self.WeaponTypes`)
        (`self.SpawnAt` _array_element _array_index)))
    (:`then_2`
      (for _index (range (`KismetArrayLibrary.Array_Length` (`self.WeaponTypes`)) (`KismetArrayLibrary.Array_Length` (`self.Locations`)))
        (`self.SpawnAt` (`KismetArrayLibrary.Array_Random` (`self.CrateTypes`)) _index)))))

(event `SpawnAt`
  (params (`Actor Type` :type "Actor Class Reference") (`Spawn Point Index` :type Integer))
  (`|SpawnActorFromClass` `Actor Type` (`self.GetTransform` (`|GetArrayItem` (`self.Locations`) `Spawn Point Index`)) "Undefined" "MultiplyWithRoot" null null))

(fn `UserConstructionScript`)
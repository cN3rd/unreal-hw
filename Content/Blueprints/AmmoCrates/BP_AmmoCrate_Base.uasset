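; Base ammo crate pickup that gives the player ammo for one weapon type.
; On BeginPlay it rolls a random amount between its min and max and displays it on a WBP_AmmoCount widget component.
; When the player pawn enters the sphere, interface messages check that it has a matching weapon that can accept ammo, then add the amount and destroy the crate.
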(event `self.ReceiveBeginPlay`
  (`|ExecutionSequence`
    (:`then_0`
      (bind _output_get (set `self.AmmoAmount` (`KismetMathLibrary.RandomIntegerInRange` (`self.AmmoMin`) (`self.AmmoMax`)))))
    (:`then_1`
      (bind _aswbp_ammo_count (cast `/Game/UI/Blueprints/WBP_AmmoCount` (`WidgetComponent.GetWidget` (`self.AmmoCountWidget`))))
      (`/Game/UI/Blueprints/WBP_AmmoCount.SetAmmoAmount` _aswbp_ammo_count _output_get))))

(event `self.Sphere.OnComponentBeginOverlap`
  (params (OverlappedComponent :type "PrimitiveComponent Object Reference") (OtherActor :type "Actor Object Reference") (OtherComp :type "PrimitiveComponent Object Reference") (OtherBodyIndex :type Integer) (bFromSweep :type Boolean) (SweepResult :type "HitResult Structure (by ref)"))
  (bind _returnvalue (`GameplayStatics.GetPlayerPawn` 0))
  (bind _ammotype (`self.AmmoType`))
  (bind _hasweapon (message `/Game/Blueprints/Interfaces/BPI_Player.HasWeaponOfType` _returnvalue _ammotype))
  (bind _canaddammo (message `/Game/Blueprints/Interfaces/BPI_Player.CanAddAmmoIntoWeapon` _returnvalue _ammotype 0))
  (if (and _hasweapon _canaddammo (== OtherActor _returnvalue))
    ;[1 1 1] Add new ammo
    (message `/Game/Blueprints/Interfaces/BPI_Player.AddAmmoIntoWeapon` _returnvalue (`self.AmmoType`) (`self.AmmoAmount`))
    (`self.K2_DestroyActor`)))

(fn `UserConstructionScript`)
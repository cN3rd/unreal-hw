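; Guard character that patrols, chases players and attacks with a baton, with a linked health widget.
; An enum state gates behavior as AIMoveTo loops through path points or pursues the player.
; Detection-sphere overlap starts a timeline-driven eye trace, where any hit triggers a faster chase that reverts to patrol when a move fails out of range.
; Hit reduces health, triggers stagger or death states and returns a larger value on death.
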(event `self.ReceiveBeginPlay`
  (bind _aswbp_guard_health (cast `/Game/UI/Blueprints/WBP_GuardHealth` (`WidgetComponent.GetWidget` (`self.GuardHealthWidget`))))
  (set `/Game/UI/Blueprints/WBP_GuardHealth.Guard` self _aswbp_guard_health)
  (`self.Do Patrol`))

(event `Do Patrol`
  (`|ExecutionSequence`
    (:`then_0`
      (set `self.Current State` "NewEnumerator0")
      (`KismetSystemLibrary.Delay` 2.0)
      (`self.Set Patrol Speed`))
    (:`then_1`
      (set `self.Current State` "NewEnumerator1")
      (`|AIMoveTo` self (0.0 0.0 0.0) (`|GetArrayItem` (`self.PatrolPath`) (`self.Current Path Point`))
        (:`OnSuccess`
          (`KismetSystemLibrary.Delay` 3.0)
          (set `self.Current Path Point` (mod (+ (`self.Current Path Point`) 1) (`KismetArrayLibrary.Array_Length` (`self.PatrolPath`))))
          (`self.Do Patrol`))))))

(event `Do Hit Animation`
  (set `self.Current State` "NewEnumerator3")
  (`MovementComponent.StopMovementImmediately` (`self.CharacterMovement`))
  (`KismetSystemLibrary.Delay` 3.0))

(event `Do Death`
  (set `self.Current State` "NewEnumerator4"))

(event `Set Patrol Speed`
  (set `CharacterMovementComponent.MaxWalkSpeed` 150.0 (`self.CharacterMovement`)))

(event `Set Chase Speed`
  (set `CharacterMovementComponent.MaxWalkSpeed` 600.0 (`self.CharacterMovement`)))

(event `self.BatonCollider.OnComponentBeginOverlap`
  (params (OverlappedComponent :type "PrimitiveComponent Object Reference") (OtherActor :type "Actor Object Reference") (OtherComp :type "PrimitiveComponent Object Reference") (OtherBodyIndex :type Integer) (bFromSweep :type Boolean) (SweepResult :type "HitResult Structure (by ref)"))
  (if (and (`KismetSystemLibrary.DoesImplementInterface` OtherActor "/Game/Blueprints/Interfaces/BPI_Player.BPI_Player_C") (`|EnumEquality` (`self.Current State`) "NewEnumerator2"))
    (message `/Game/Blueprints/Interfaces/BPI_HittableActor.Hit` OtherActor 0)))

(event `self.DetectionSphere.OnComponentEndOverlap`
  (params (OverlappedComponent :type "PrimitiveComponent Object Reference") (OtherActor :type "Actor Object Reference") (OtherComp :type "PrimitiveComponent Object Reference") (OtherBodyIndex :type Integer))
  (if (`KismetSystemLibrary.DoesImplementInterface` OtherActor "/Game/Blueprints/Interfaces/BPI_Player.BPI_Player_C")
    (if (`|EnumEquality` (`self.Current State`) "NewEnumerator5")
      (`KismetSystemLibrary.PrintString` "Still in chase")
      (else
        (set `self.Is Player In Range` false)
        (set `self.Chased Player` null)))))

(event `self.DetectionSphere.OnComponentBeginOverlap`
  (params (OverlappedComponent :type "PrimitiveComponent Object Reference") (OtherActor :type "Actor Object Reference") (OtherComp :type "PrimitiveComponent Object Reference") (OtherBodyIndex :type Integer) (bFromSweep :type Boolean) (SweepResult :type "HitResult Structure (by ref)"))
  (if (`KismetSystemLibrary.DoesImplementInterface` OtherActor "/Game/Blueprints/Interfaces/BPI_Player.BPI_Player_C")
    (if (`self.Is Player In Range`)
      (`self.Do Chase`)
      (else
        (set `self.Is Player In Range` true)
        (set `self.Chased Player` OtherActor)
        (`self.Do Line Trace Chase`)))))

(event `Look At Player Chase`
  (`MovementComponent.StopMovementImmediately` (`self.CharacterMovement`))
  (bind (_direction _time) (`Timeline|Timeline`)
    (:`Update`
      (`self.K2_SetActorRotation` (`KismetMathLibrary.RLerp` (`self.K2_GetActorRotation`) (`KismetMathLibrary.FindLookAtRotation` (`self.K2_GetActorLocation`) (`self.K2_GetActorLocation`)) _time true)))
    (:`Finished`
      (`self.Do Line Trace Chase`))))

(event `Do Line Trace Chase`
  (bind _eyes (`self.Eyes`))
  (bind _returnvalue (`SceneComponent.K2_GetComponentLocation` _eyes))
  (`KismetSystemLibrary.PrintString` "Looking for player")
  (`MovementComponent.StopMovementImmediately` (`self.CharacterMovement`))
  (set `self.Current State` "NewEnumerator0")
  (`Timeline|LookAt Timeline`
    (:`Update`
      (bind (_outhit _returnvalue_2) (`KismetSystemLibrary.LineTraceSingle` :`Start` _returnvalue :`End` (+ _returnvalue (* (`SceneComponent.GetForwardVector` _eyes) (`SphereComponent.GetScaledSphereRadius` (`self.DetectionSphere`)))) :`TraceChannel` "TraceTypeQuery1" :`DrawDebugType` "ForDuration"))
      (`KismetSystemLibrary.PrintString` (`KismetStringLibrary.Conv_BoolToString` _returnvalue_2))
      (if _returnvalue_2
        (`TimelineComponent.Stop` (`self.LookAt Timeline`))
        (`self.Do Chase`)))))

(event `Do Chase`
  (`KismetSystemLibrary.PrintString` "Start Chase")
  (set `self.Current State` "NewEnumerator5")
  (`self.Set Chase Speed`)
  (`|AIMoveTo` self (0.0 0.0 0.0) (`self.Chased Player`)
    (:`OnSuccess`
      (`KismetSystemLibrary.Delay` 0.5)
      (set `self.Current State` "NewEnumerator2")
      (`KismetSystemLibrary.Delay` 3.0)
      (`self.Do Chase` :!label _label))
    (:`OnFail`
      (`KismetSystemLibrary.Delay` 3.0)
      (if (`self.Is Player In Range`)
        (goto _label)
        (else
          (`self.Give Up Patrol`))))))

(event `Give Up Patrol`
  (`KismetSystemLibrary.PrintString` "Giving up Chase")
  (set `self.Is Player In Range` false)
  (set `self.Chased Player` null)
  (`self.Do Patrol`))

(fn `Hit`
  (params (Damage :type Integer))
  (returns (XPReward :type Integer))
  (bind _output_get (set `self.Health` (`KismetMathLibrary.Clamp` (- (`self.Health`) Damage) 0 (`self.MaxHealth`))))
  (if (<= _output_get 0)
    (`self.Do Death`)
    (return 50)
    (else
      (`self.Do Hit Animation`)
      (return 5))))

(fn `UserConstructionScript`)
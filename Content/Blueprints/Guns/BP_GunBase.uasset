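; Base gun Blueprint that manages a clamped ammo count and fires physical bullet projectiles.
; Shoot spawns a scaled-down BP_Bullet at the barrel pivot with the gun's damage, pushes it forward by impulse and decrements ammo.
; It binds to each bullet's hit event, which only prints the XP reward.
; AddAmmo clamps to the maximum, and CanAddAmmoIntoWeapon returns false whenever the new total would reach or exceed it.
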(event `/Game/Blueprints/Interfaces/BPI_Gun.AddAmmo`
  (params (Ammo :type Integer))
  (bind _output_get (set `self.Ammo` (`KismetMathLibrary.Clamp` (+ Ammo (`self.Ammo`)) 0 (`self.MaxAmmo`))))
  (`KismetSystemLibrary.PrintString` (`KismetTextLibrary.Conv_TextToString` (`|FormatText` "{GunType} now has {Ammo} ammo" (`|GetEnumeratorNameAsString` (`self.Weapon Type`)) _output_get))))

(event `/Game/Blueprints/Interfaces/BPI_Gun.Shoot`
  (if (> (`self.Ammo`) 0)
    (bind _returnvalue (`|SpawnActorFromClass` "/Game/Blueprints/Guns/BP_Bullet.BP_Bullet_C" (`KismetMathLibrary.MakeTransform` (`SceneComponent.K2_GetComponentLocation` (`self.BarrelPivot`)) (struct) (0.1 0.1 0.1)) "Undefined" "MultiplyWithRoot" null (`self.BulletDamage`) null))
    (`|ExecutionSequence`
      (:`then_0`
        (`PrimitiveComponent.AddImpulse` (`/Game/Blueprints/Guns/BP_Bullet.Sphere` _returnvalue) (* (`SceneComponent.GetForwardVector` (`self.BarrelPivot`)) 1000.0) "None" false)
        (`/Engine/EditorBlueprintResources/StandardMacros.DecrementInt` (`self.Ammo`)))
      (:`then_1`
        (add `/Game/Blueprints/Guns/BP_Bullet.OnBulletHit` _returnvalue (delegate `CustomEvent`))))
    (else
      (`KismetSystemLibrary.PrintString` "No bullets!"))))

(event `CustomEvent`
  (params (XPReward :type Integer))
  (`KismetSystemLibrary.PrintString` (`KismetStringLibrary.Concat_StrStr` "Player get XP:  " (`KismetStringLibrary.Conv_IntToString` XPReward))))

(fn `CanAddAmmoIntoWeapon`
  (params (NewAmmo :type Integer))
  (returns (CanAddAmmo :type Boolean))
  (return (!= (`KismetMathLibrary.Clamp` (+ NewAmmo (`self.Ammo`)) 0 (`self.MaxAmmo`)) (`self.MaxAmmo`))))

(fn `GetAmmo`
  (returns (AmmoCount :type Integer))
  (return (`self.Ammo`)))

(fn `GetMaxAmmo`
  (returns (AmmoCount :type Integer))
  (return (`self.MaxAmmo`)))

(fn `UserConstructionScript`
  (`parent.UserConstructionScript`))